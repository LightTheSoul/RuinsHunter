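; BP_ComboNofity is an animation notify state that controls which attacks the player has available during a window in an animation.
; On begin, it passes its LightAttacks and HeavyAttacks values to BP_Player's AttackTypes, and on end it calls DefaultAttack.
; Both events fetch the player character at index 0 rather than the mesh owner, and do nothing if the cast to BP_Player fails.
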(fn ReceivedNotifyBegin
  (params (MeshComp :type Skeletal%20Mesh%20Component%20Object%20Reference) (Animation :type Anim%20Sequence%20Base%20Object%20Reference) (TotalDuration :type Float%20%28single-precision%29) (EventReference :type Anim%20Notify%20Event%20Reference%20Structure%20%28by%20ref%29))
  (bind _asbp_player (Utilities|Casting|CastToBP_Player (Game|GetPlayerCharacter MeshComp)))
  (Default|AttackTypes _asbp_player (Variables|Default|GetLight%20Attacks) (Variables|Default|GetHeavy%20Attacks))
  (return true))

(fn ReceivedNotifyEnd
  (params (MeshComp :type Skeletal%20Mesh%20Component%20Object%20Reference) (Animation :type Anim%20Sequence%20Base%20Object%20Reference) (EventReference :type Anim%20Notify%20Event%20Reference%20Structure%20%28by%20ref%29))
  (bind _asbp_player (Utilities|Casting|CastToBP_Player (Game|GetPlayerCharacter MeshComp)))
  (Default|DefaultAttack _asbp_player)
  (return true))