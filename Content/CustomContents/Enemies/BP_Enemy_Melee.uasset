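; BP_Enemy_Melee is a sword-wielding melee enemy that implements the attack, equip and unequip events with montages.
; Equip and unequip montage notifies time the sword's spawn and attachment to the right-hand socket, or its destruction, and update the wielding flag.
; Montage completion fires the matching event dispatchers, and the attack also signals its end when interrupted, unlike equip and unequip.
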(event EventEquipWeapon
  (bind _notifyname (Animation|Montage|PlayMontage (Variables|Character|GetMesh) "/Game/CustomContents/Animations/Sword/Equip_Sword_Montage.Equip_Sword_Montage")
    (:OnCompleted
      (Default|CallOnEquipWeapon))
    (:OnNotifyBegin
      (switch name _notifyname
        (:EquipSword
          (bind _returnvalue (Game|SpawnActorfromClass "/Game/CustomContents/Weapons/BP_Weapon_Sword.BP_Weapon_Sword_C" (Transformation|GetActorTransform) "Undefined" "MultiplyWithRoot" 0 0))
          (bind _output_get (Variables|Default|SetWeaponActor _returnvalue))
          (Transformation|AttachComponentToComponent _output_get (Variables|Character|GetMesh) "hand_r_sword_socket" "SnapToTarget" "SnapToTarget" "SnapToTarget" true)
          (Variables|Default|SetIsWieldingWeapon true))))))

(event EventUnEquipWeapon
  (bind _notifyname (Animation|Montage|PlayMontage (Variables|Character|GetMesh) "/Game/CustomContents/Animations/Sword/UnEquip_Sword_Montage.UnEquip_Sword_Montage")
    (:OnCompleted
      (Default|CallOnUnEquipWeapon))
    (:OnNotifyBegin
      (switch name _notifyname
        (:UnEquipSword
          (Actor|DestroyActor (Variables|Default|GetWeaponActor))
          (Variables|Default|SetIsWieldingWeapon false))))))

(event EventAttack
  (Animation|Montage|PlayMontage (Variables|Character|GetMesh) "/Game/CustomContents/Animations/Sword/Sword_Slash_Montage.Sword_Slash_Montage"
    (:OnCompleted
      _)
    (:OnInterrupted
      _))
  (Default|CallOnAttackEnd))

(fn ConstructionScript
  (|CallParentFunction))