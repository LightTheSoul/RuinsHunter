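; Second boss enemy Blueprint that overrides weapon equip and unequip as stand-up and kneel transitions.
; EquipWeapon plays the kneel-end montage while spawning the boss weapon and a hidden knife onto mesh sockets, clearing BossKneel after a short delay.
; UnEquipWeapon plays the kneel-begin montage, sets BossKneel, and clears IsWieldingWeapon on completion without destroying the spawned actors.
; Both fire their equip or unequip dispatcher when the montage completes.
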(event EventBeginPlay
  (|CallParentFunction) ; This node is disabled and will not be called.\nDrag off pins to build functionality.
)

(event EventUnEquipWeapon
  ;[1 1 1 1 40] Equip Unequip
  (Animation|Montage|PlayMontage (Variables|Character|GetMesh) "/Game/CustomContents/Animations/AssetAnimations/2H_Kneel/MON/2H_Kneel_Begin_Seq_Montage.2H_Kneel_Begin_Seq_Montage"
    (:then
      (Variables|Default|SetBossKneel true))
    (:OnCompleted
      (Default|CallOnUnEquipWeapon)
      (Variables|Default|SetIsWieldingWeapon false))))

(event EventEquipWeapon
  ;[1 1 1 1 40] Equip Unequip
  (Animation|Montage|PlayMontage (Variables|Character|GetMesh) "/Game/CustomContents/Animations/AssetAnimations/2H_Kneel/MON/2H_Kneel_End_Seq_Montage.2H_Kneel_End_Seq_Montage"
    (:then
      (bind _returnvalue (Game|SpawnActorfromClass "/Game/CustomContents/Weapons/BP_Weapon_Boss.BP_Weapon_Boss_C" (Math|Transform|MakeTransform "0, 0, 0" "0, 0, 0" "1.000000,1.000000,1.000000") "Undefined" "MultiplyWithRoot" 0 0))
      (bind _output_get (Variables|Default|SetWeaponActor _returnvalue))
      (Transformation|AttachComponentToComponent _output_get (Variables|Character|GetMesh) "weapon_r" "SnapToTarget" "SnapToTarget" "SnapToTarget" true)
      (Variables|Default|SetIsWieldingWeapon true)
      (bind _returnvalue_2 (Game|SpawnActorfromClass "/Game/CustomContents/Weapons/BP_Knife.BP_Knife_C" (Math|Transform|MakeTransform "0, 0, 0" "0, 0, 0" "1.000000,1.000000,1.000000") "Undefined" "MultiplyWithRoot" 0 0))
      (bind _output_get_2 (Variables|Default|SetBPKnife _returnvalue_2))
      (Transformation|AttachComponentToComponent _output_get_2 (Variables|Character|GetMesh) "knife_boss" "SnapToTarget" "SnapToTarget" "SnapToTarget" true)
      (Rendering|SetVisibility (Variables|/Game/CustomContents/Weapons/BP_Knife.BP_Knife_C|GetSkeletalMesh (Variables|Default|GetBPKnife)) false false)
      (Utilities|FlowControl|Delay 0.2)
      (Variables|Default|SetBossKneel false))
    (:OnCompleted
      (Default|CallOnEquipWeapon))))

(fn ConstructionScript
  (|CallParentFunction))