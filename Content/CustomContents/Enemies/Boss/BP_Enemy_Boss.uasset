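; Boss enemy Blueprint that starts kneeling, creates a boss health bar and win screen widget, and has its max health set in construction.
; Equip and unequip play kneel montages, with equip spawning a two-handed weapon and a hidden knife on mesh sockets.
; Attack events feed montages and damage info to BPCAttacks for slash, smash and jump-smash moves.
; The ranged attack uses montage notifies to throw a knife projectile that deals damage on impact.
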(event Custom|Attack2Combo2
  (params (AttackTarget :type Actor%20Object%20Reference))
  ;[1 1 1 1 40] Attacks
  (Default|SlashMeleeAttack (Variables|Default|GetBPC_Attacks) (Utilities|Struct|MakeS_AttackInfo AttackTarget "/Game/CustomContents/Animations/AssetAnimations/2H_Sword_Attack/MON/Enemy_Boss/2H_Attack_2Combo_02.2H_Attack_2Combo_02" (Utilities|Struct|MakeS_DamageInfo 1e+01 "NewEnumerator1" "NewEnumerator1" false true true)) 1e+02 3e+02))

(event Custom|AttackRange
  (params (AttackTarget :type Actor%20Object%20Reference))
  ;[1 1 1 1 40] Attacks
  (CallFunction|Attack AttackTarget)
  (bind _notifyname (Animation|Montage|PlayMontage (Variables|Character|GetMesh) "/Game/CustomContents/Animations/AssetAnimations/2H_Sword_Attack/MON/Enemy_Boss/SSH_KnifeAttack.SSH_KnifeAttack")
    (:OnCompleted
      (CallFunction|AttackEnd AttackTarget))
    (:OnNotifyBegin
      (switch name _notifyname
        (:Throw
          (Rendering|SetVisibility (Variables|/Game/CustomContents/Weapons/BP_Knife.BP_Knife_C|GetSkeletalMesh (Variables|Default|GetBPKnife)) false false)
          (bind _returnvalue (Game|SpawnActorfromClass "/Game/CustomContents/Projectile/BP_Projectile_Knife.BP_Projectile_Knife_C" (Math|Transform|MakeTransform (Transformation|GetSocketLocation (Variables|Character|GetMesh) "knife_boss") (Math|Rotator|CombineRotators (Transformation|GetActorRotation AttackTarget) "0.000000,180.000000,0.000000") "1.000000,1.000000,1.000000") "Undefined" "MultiplyWithRoot" self 6e+03 0.0 AttackTarget true self))
          (EventDispatchers|AssignOnPrejectileImpact _returnvalue (delegate Custom|OnPrejectileImpact_Event))
          (Collision|IgnoreActorwhenMoving (Variables|Default|GetCapsuleComponent) _returnvalue true))
        (:Equip
          (Rendering|SetVisibility (Variables|/Game/CustomContents/Weapons/BP_Knife.BP_Knife_C|GetSkeletalMesh (Variables|Default|GetBPKnife)) true false))))))

(event Custom|HeavyAttack
  (params (AttackTarget :type Actor%20Object%20Reference))
  (Default|SlashMeleeAttack (Variables|Default|GetBPC_Attacks) (Utilities|Struct|MakeS_AttackInfo AttackTarget "/Game/CustomContents/Animations/AssetAnimations/2H_Sword_Attack/MON/Enemy_Boss/HeavyAttack.HeavyAttack" (Utilities|Struct|MakeS_DamageInfo 1e+01 "NewEnumerator1" "NewEnumerator1" false true true)) 2e+02 3e+02))

(event Custom|DodgeLAttack
  (params (AttackTarget :type Actor%20Object%20Reference))
  (Default|SlashMeleeAttack (Variables|Default|GetBPC_Attacks) (Utilities|Struct|MakeS_AttackInfo AttackTarget "/Game/CustomContents/Animations/AssetAnimations/2H_Sword_Attack/MON/Enemy_Boss/DodgeLAttack.DodgeLAttack" (Utilities|Struct|MakeS_DamageInfo 1e+01 "NewEnumerator1" "NewEnumerator1" false true true)) 2e+02 3e+02))

(event Custom|DodgeRAttack
  (params (AttackTarget :type Actor%20Object%20Reference))
  (Default|SlashMeleeAttack (Variables|Default|GetBPC_Attacks) (Utilities|Struct|MakeS_AttackInfo AttackTarget "/Game/CustomContents/Animations/AssetAnimations/2H_Sword_Attack/MON/Enemy_Boss/DodgeRAttack.DodgeRAttack" (Utilities|Struct|MakeS_DamageInfo 1e+01 "NewEnumerator1" "NewEnumerator1" false true true)) 2e+02 3e+02))

(event Custom|AttackJump
  (params (AttackTarget :type Actor%20Object%20Reference))
  ;[1 1 1 1 40] Attacks
  (Default|JumpSmashMeleeAttack (Variables|Default|GetBPC_Attacks) (Utilities|Struct|MakeS_AttackInfo AttackTarget "/Game/CustomContents/Animations/AssetAnimations/2H_Sword_Attack/MON/Enemy_Boss/2Hand_Attack_Jump_Montage.2Hand_Attack_Jump_Montage" (Utilities|Struct|MakeS_DamageInfo 1e+01 "NewEnumerator1" "NewEnumerator2")) 1e+03))

(event Custom|OnPrejectileImpact_Event
  (params (OtherActor :type Actor%20Object%20Reference) (Hit :type Hit%20Result%20Structure))
  ;[1 1 1 1 40] Attacks
  (Class|BPIDamageable|TakeDamage(Message) OtherActor (Utilities|Struct|MakeS_DamageInfo 2e+01 "NewEnumerator2" "NewEnumerator3" false true true) self))

(event Custom|DefaultAttack
  (params (AttackTarget :type Actor%20Object%20Reference))
  ;[1 1 1 1 40] Attacks
  (Default|SlashMeleeAttack (Variables|Default|GetBPC_Attacks) (Utilities|Struct|MakeS_AttackInfo AttackTarget "/Game/CustomContents/Animations/AssetAnimations/2H_Sword_Attack/MON/Enemy_Boss/Mon_Boss/2H_Attack_05_Seq_Montage.2H_Attack_05_Seq_Montage" (Utilities|Struct|MakeS_DamageInfo 1e+01 "NewEnumerator1" "NewEnumerator1" false true true)) 1e+02 3e+02))

(event Custom|Attack3Combo1
  (params (AttackTarget :type Actor%20Object%20Reference))
  ;[1 1 1 1 40] Attacks
  (Default|SlashandSmashMeleeAttack (Variables|Default|GetBPC_Attacks) (Utilities|Struct|MakeS_AttackInfo AttackTarget "/Game/CustomContents/Animations/AssetAnimations/2H_Sword_Attack/MON/Enemy_Boss/2H_Attack_3Combo_01.2H_Attack_3Combo_01" (Utilities|Struct|MakeS_DamageInfo 1e+01 "NewEnumerator1" "NewEnumerator1" false true true)) 8e+02 1e+02 3e+02))

(event Custom|SingleAttack
  (params (AttackTarget :type Actor%20Object%20Reference))
  (Default|JumpSmashMeleeAttack (Variables|Default|GetBPC_Attacks) (Utilities|Struct|MakeS_AttackInfo AttackTarget "/Game/CustomContents/Animations/AssetAnimations/2H_Sword_Attack/MON/Enemy_Boss/SingleAttack.SingleAttack" (Utilities|Struct|MakeS_DamageInfo 1e+01 "NewEnumerator1" "NewEnumerator2")) 5e+02))

(event Custom|AttackCharge
  (params (AttackTarget :type Actor%20Object%20Reference))
  ;[1 1 1 1 40] Attacks
  (Default|SmashMeleeAttack (Variables|Default|GetBPC_Attacks) (Utilities|Struct|MakeS_AttackInfo AttackTarget "/Game/CustomContents/Animations/AssetAnimations/2H_Sword_Attack/MON/Enemy_Boss/KnockBack_Attack_Montage.KnockBack_Attack_Montage" (Utilities|Struct|MakeS_DamageInfo 25.0 "NewEnumerator1" "NewEnumerator2")) 1.2e+03))

(event Custom|Attack2Combo1
  (params (AttackTarget :type Actor%20Object%20Reference))
  ;[1 1 1 1 40] Attacks
  (Default|SlashMeleeAttack (Variables|Default|GetBPC_Attacks) (Utilities|Struct|MakeS_AttackInfo AttackTarget "/Game/CustomContents/Animations/AssetAnimations/2H_Sword_Attack/MON/Enemy_Boss/2H_Attack_2Combo_01.2H_Attack_2Combo_01" (Utilities|Struct|MakeS_DamageInfo 1e+01 "NewEnumerator1" "NewEnumerator1" false true true)) 1e+02 3e+02))

(event Custom|AiSlashAttackCombo
  (params (AttackTarget :type Actor%20Object%20Reference))
  (Default|SlashMeleeAttack (Variables|Default|GetBPC_Attacks) (Utilities|Struct|MakeS_AttackInfo AttackTarget "/Game/CustomContents/Animations/AssetAnimations/2H_Sword_Attack/MON/Enemy_Boss/BossAiSlashAttackCombo.BossAiSlashAttackCombo" (Utilities|Struct|MakeS_DamageInfo 1e+01 "NewEnumerator1" "NewEnumerator1" false false false)) 1e+02 3e+02))

(event Custom|Attack3Combo2
  (params (AttackTarget :type Actor%20Object%20Reference))
  ;[1 1 1 1 40] Attacks
  (Default|SlashandSmashMeleeAttack (Variables|Default|GetBPC_Attacks) (Utilities|Struct|MakeS_AttackInfo AttackTarget "/Game/CustomContents/Animations/AssetAnimations/2H_Sword_Attack/MON/Enemy_Boss/2H_Attack_3Combo_02.2H_Attack_3Combo_02" (Utilities|Struct|MakeS_DamageInfo 1e+01 "NewEnumerator1" "NewEnumerator1" false true true)) 6e+02 1e+02 3e+02))

(event EventBeginPlay
  (|CallParentFunction)
  ;[1 1 1 1 40] Health Widget
  (Variables|Default|SetBossKneel true)
  (UserInterface|SetWidget (Variables|Default|GetHealthBar) 0)
  (bind _returnvalue (UserInterface|CreateWidget "/Game/CustomContents/Widget/W_BossHealthBar.W_BossHealthBar_C" 0 self))
  (Variables|Default|SetBossHealthbarWidgetRef _returnvalue)
  (bind _returnvalue_2 (UserInterface|CreateWidget "/Game/CustomContents/MainMenu/NewUI/UI_NewGameWin.UI_NewGameWin_C"))
  (Variables|Default|SetEnemyFelledUI _returnvalue_2))

(event EventUnEquipWeapon
  ;[1 1 1 1 40] Equip Unequip
  (Animation|Montage|PlayMontage (Variables|Character|GetMesh) "/Game/CustomContents/Animations/AssetAnimations/2H_Kneel/MON/2H_Kneel_Begin_Seq_Montage.2H_Kneel_Begin_Seq_Montage"
    (:then
      (Variables|Default|SetBossKneel true))
    (:OnCompleted
      (Default|CallOnUnEquipWeapon)
      (Variables|Default|SetIsWieldingWeapon false))))

(event EventEquipWeapon
  ;[1 1 1 1 40] Equip Unequip
  (Animation|Montage|PlayMontage (Variables|Character|GetMesh) "/Game/CustomContents/Animations/AssetAnimations/2H_Kneel/MON/2H_Kneel_End_Seq_Montage.2H_Kneel_End_Seq_Montage"
    (:then
      (bind _returnvalue (Game|SpawnActorfromClass "/Game/CustomContents/Weapons/BP_Weapon_Boss.BP_Weapon_Boss_C" (Math|Transform|MakeTransform "0, 0, 0" "0, 0, 0" "1.000000,1.000000,1.000000") "Undefined" "MultiplyWithRoot" 0 0))
      (bind _output_get (Variables|Default|SetWeaponActor _returnvalue))
      (Transformation|AttachComponentToComponent _output_get (Variables|Character|GetMesh) "weapon_r" "SnapToTarget" "SnapToTarget" "SnapToTarget" true)
      (Variables|Default|SetIsWieldingWeapon true)
      (bind _returnvalue_2 (Game|SpawnActorfromClass "/Game/CustomContents/Weapons/BP_Knife.BP_Knife_C" (Math|Transform|MakeTransform "0, 0, 0" "0, 0, 0" "1.000000,1.000000,1.000000") "Undefined" "MultiplyWithRoot" 0 0))
      (bind _output_get_2 (Variables|Default|SetBPKnife _returnvalue_2))
      (Transformation|AttachComponentToComponent _output_get_2 (Variables|Character|GetMesh) "knife_boss" "SnapToTarget" "SnapToTarget" "SnapToTarget" true)
      (Rendering|SetVisibility (Variables|/Game/CustomContents/Weapons/BP_Knife.BP_Knife_C|GetSkeletalMesh (Variables|Default|GetBPKnife)) false false)
      (Utilities|FlowControl|Delay 0.2)
      (Variables|Default|SetBossKneel false))
    (:OnCompleted
      (Default|CallOnEquipWeapon))))

(fn ConstructionScript
  (bind _bpc_damagesystem (Variables|Default|GetBPC_DamageSystem))
  (|CallParentFunction)
  (bind _output_get (Variables|/Game/CustomContents/DamageSystem/BPC_DamageSystem.BPC_DamageSystem_C|SetMaxHealth _bpc_damagesystem 1e+03))
  (Variables|/Game/CustomContents/DamageSystem/BPC_DamageSystem.BPC_DamageSystem_C|SetHealth _bpc_damagesystem _output_get))