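; BP_Enemy_Mage is a mage enemy Blueprint that defines a casting attack, its preferred combat ranges and its movement speeds.
; Attack plays a casting montage on the mesh, with Notify Begin feeding a switch that has no actions wired to it.
; GetIdealRange supplies fixed attack and defend radii, and SetMovementSpeed maps each movement state from idle to sprinting to a speed value.
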(event EventBeginPlay
  (|CallParentFunction) ; This node is disabled and will not be called.\nDrag off pins to build functionality.
)

(event EventAttack
  (params (AttackTarget :type Actor%20Object%20Reference))
  (bind _notifyname (Animation|Montage|PlayMontage (Variables|Character|GetMesh) "/Game/CustomContents/Animations/Sword/Sword_Casting_Montage.Sword_Casting_Montage")
    (:OnNotifyBegin
      (switch name _notifyname))))

(fn ConstructionScript
  (|CallParentFunction))

(fn GetIdealRange
  (return 5e+02 7e+02))

(fn SetMovementSpeed
  (params (Speed :type E_MovementSpeed%20Enum :default "NewEnumerator0"))
  (return (Utilities|Select :Index Speed :NewEnumerator0 0.0 :NewEnumerator1 1.5e+02 :NewEnumerator2 2.5e+02 :NewEnumerator3 4e+02)))