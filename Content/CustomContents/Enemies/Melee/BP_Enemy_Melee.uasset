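; Melee enemy character that fights with a two-handed sword, built on a parent enemy Blueprint.
; Equip and unequip play draw and sheathe montages, spawning and attaching or destroying the sword on montage notifies, then signal completion.
; Basic, combo and strong attacks pass montage and damage info to BPCAttacks as slash or area smash attacks.
; It also supplies ideal attack and defend ranges and caches the mesh's initial rotation.
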(event Custom|StrongAttack
  (params (AttackTarget :type Actor%20Object%20Reference))
  ;[0 0 0] Attack
  (Default|SmashMeleeAttack (Variables|Default|GetBPC_Attacks) (Utilities|Struct|MakeS_AttackInfo AttackTarget "/Game/CustomContents/Animations/AssetAnimations/2H_Sword_Attack/MON/BaseSword/2H_Attack_Strong_01.2H_Attack_Strong_01" (Utilities|Struct|MakeS_DamageInfo 1e+01 "NewEnumerator3")) 3e+02))

(event Custom|BasicAttack1
  (params (AttackTarget :type Actor%20Object%20Reference))
  ;[0 0 0] Attack
  (Default|SlashMeleeAttack (Variables|Default|GetBPC_Attacks) (Utilities|Struct|MakeS_AttackInfo AttackTarget "/Game/CustomContents/Animations/AssetAnimations/2H_Sword_Attack/MON/BaseSword/2H_Attack_Basic_01.2H_Attack_Basic_01" (Utilities|Struct|MakeS_DamageInfo 1e+01 "NewEnumerator1")) 2e+01 2e+02))

(event Custom|BasicAttack2
  (params (AttackTarget :type Actor%20Object%20Reference))
  ;[0 0 0] Attack
  (Default|SlashMeleeAttack (Variables|Default|GetBPC_Attacks) (Utilities|Struct|MakeS_AttackInfo AttackTarget "/Game/CustomContents/Animations/AssetAnimations/2H_Sword_Attack/MON/BaseSword/2H_Attack_Basic_02.2H_Attack_Basic_02" (Utilities|Struct|MakeS_DamageInfo 1e+01 "NewEnumerator1")) 2e+01 2e+02))

(event Custom|ComboAttack
  (params (AttackTarget :type Actor%20Object%20Reference))
  ;[0 0 0] Attack
  (Default|SlashMeleeAttack (Variables|Default|GetBPC_Attacks) (Utilities|Struct|MakeS_AttackInfo AttackTarget "/Game/CustomContents/Animations/AssetAnimations/2H_Sword_Attack/MON/BaseSword/2H_Attack_Combo_01.2H_Attack_Combo_01" (Utilities|Struct|MakeS_DamageInfo 1e+01 "NewEnumerator1")) 2e+01 2e+02))

(event EventEquipWeapon
  ;[0 0 0] EquipWeapon
  (bind _notifyname (Animation|Montage|PlayMontage (Variables|Character|GetMesh) "/Game/CustomContents/Animations/AssetAnimations/2H_Sword_Equip/MON/2H_Sword_Unsheathe_Back_Seq_Montage.2H_Sword_Unsheathe_Back_Seq_Montage")
    (:OnCompleted
      (Default|CallOnEquipWeapon))
    (:OnNotifyBegin
      (switch name _notifyname
        (:EquipSword
          (bind _returnvalue (Game|SpawnActorfromClass "/Game/CustomContents/Weapons/BP_Weapon_Sword.BP_Weapon_Sword_C" (Transformation|GetActorTransform) "Undefined" "MultiplyWithRoot" 0 0))
          (bind _output_get (Variables|Default|SetWeaponActor _returnvalue))
          (Transformation|AttachComponentToComponent _output_get (Variables|Character|GetMesh) "hand_r_sword_socket" "SnapToTarget" "SnapToTarget" "SnapToTarget" true)
          (Variables|Default|SetIsWieldingWeapon true))))))

(event EventUnEquipWeapon
  ;[0 0 0] UnEquipWeapon
  (bind _notifyname (Animation|Montage|PlayMontage (Variables|Character|GetMesh) "/Game/CustomContents/Animations/AssetAnimations/2H_Sword_Equip/MON/2H_Sword_Sheathe_Back_Seq_Montage.2H_Sword_Sheathe_Back_Seq_Montage")
    (:OnCompleted
      (Default|CallOnUnEquipWeapon))
    (:OnNotifyBegin
      (switch name _notifyname
        (:UnEquipSword
          (Actor|DestroyActor (Variables|Default|GetWeaponActor))
          (Variables|Default|SetIsWieldingWeapon false))))))

(event EventBeginPlay
  (|CallParentFunction))

(fn ConstructionScript
  (|CallParentFunction)
  (Variables|Default|SetMeshRotationBeforeSpin (Variables|/Script/Engine.SceneComponent|GetRelativeRotation (Variables|Character|GetMesh))))

(fn GetIdealRange
  (return 2e+02 4e+02))