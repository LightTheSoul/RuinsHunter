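; Ranged enemy character that fights with a rifle, extending a parent enemy class's attack and equip flow.
; On BeginPlay it spawns a rifle, attaches it to the hand socket and signals that it is equipped.
; Attacks play a fire montage whose notify traces from weapon to target, dealing damage only if nothing blocks Visibility.
; It also maps movement states to walk speeds and supplies long attack and defend ranges.
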(event EventBeginPlay
  (|CallParentFunction)
  (CallFunction|EquipWeapon))

(event EventEquipWeapon
  (bind _returnvalue (Game|SpawnActorfromClass "/Game/CustomContents/Weapons/BP_Weapon_Rifle.BP_Weapon_Rifle_C" (Transformation|GetActorTransform) "Undefined" "MultiplyWithRoot" 0 0))
  (bind _output_get (Variables|Default|SetWeaponActor _returnvalue))
  (Transformation|AttachComponentToComponent _output_get (Variables|Character|GetMesh) "hand_r_rifle_socket" "SnapToTarget" "SnapToTarget" "SnapToTarget" true)
  (Variables|Default|SetIsWieldingWeapon true)
  (Default|CallOnEquipWeapon))

(event EventAttack
  (params (AttackTarget :type Actor%20Object%20Reference))
  (|CallParentFunction AttackTarget)
  (bind _notifyname (Animation|Montage|PlayMontage (Variables|Character|GetMesh) "/Game/CustomContents/Animations/Rifle/Action/MM_Rifle_Fire_Montage.MM_Rifle_Fire_Montage")
    (:OnCompleted
      (CallFunction|AttackEnd AttackTarget :!label _label))
    (:OnInterrupted
      (goto _label))
    (:OnNotifyBegin
      (switch name _notifyname
        (:Fire
          (bind _returnvalue (Collision|LineTraceByChannel (Transformation|GetActorLocation (Variables|Default|GetWeaponActor)) (Transformation|GetActorLocation AttackTarget) "TraceTypeQuery1" false 0 "ForDuration"))
          (if (not _returnvalue)
            (Class|BPIDamageable|TakeDamage(Message) AttackTarget (Utilities|Struct|MakeS_DamageInfo 2e+01 "NewEnumerator2"))))))))

(fn ConstructionScript
  (|CallParentFunction))

(fn SetMovementSpeed
  (params (Speed :type E_MovementSpeed%20Enum :default "NewEnumerator0"))
  (Variables|/Script/Engine.CharacterMovementComponent|SetMaxWalkSpeed (Variables|Character|GetCharacterMovement) (Utilities|Select :Index Speed :NewEnumerator0 0.0 :NewEnumerator1 1e+02 :NewEnumerator2 3e+02 :NewEnumerator3 5e+02))
  (return 0.0))

(fn GetIdealRange
  (return 2e+03 2e+03))