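; BP_SPLINE_MASTER is a spline tool that repeats a chosen static mesh along an editable spline in the Construction Script.
; It measures the mesh's scaled bounding box along the selected forward axis to set segment length and count.
; Each segment becomes a collision-enabled spline mesh component fitted between distances along the spline.
; Tangents are clamped to segment length to keep meshes from stretching when points move.
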(event EventBeginPlay)

(fn ConstructionScript
  (bind _returnvalue (Transformation|GetActorScale3D))
  (bind _spline (Variables|Default|GetSpline))
  (bind _spline_2 (Variables|Default|GetSpline))
  (bind _spline_mesh (Variables|Default|GetSpline%20mesh))
  (bind _returnvalue_2 (StaticMesh|GetBoundingBox _spline_mesh))
  (bind (_min _max) (Utilities|Struct|BreakBox _returnvalue_2))
  (bind _returnvalue_3 (- _max _min))
  (bind _returnvalue_4 (* _returnvalue_3 _returnvalue))
  (bind (_x _y _z) (Math|Vector|BreakVector _returnvalue_4))
  ;[1 1 1] What Axis you use?
  (if (Utilities|Enum|Equal(Enum) (Variables|Default|GetForward%20Axis) "X")
    (Variables|Default|SetMesh_length%20%28auto%20detect%29 _x)
    (elif (Utilities|Enum|Equal(Enum) (Variables|Default|GetForward%20Axis) "Y")
      (Variables|Default|SetMesh_length%20%28auto%20detect%29 _y)
      (else
        (Variables|Default|SetMesh_length%20%28auto%20detect%29 _z))))
  (for _index (range 0 (Math|Float|Truncate (/ (Spline|GetSplineLength (Variables|Default|GetSpline)) (Variables|Default|GetMesh_length%20%28auto%20detect%29))))
    (bind _returnvalue_5 (AddComponent|AddSplineMeshComponent false))
    (Components|StaticMesh|SetStaticMesh _returnvalue_5 (Variables|Default|GetSpline%20mesh))
    (SplineMesh|SetForwardAxis _returnvalue_5 (Variables|Default|GetForward%20Axis) true)
    (Collision|SetCollisionEnabled _returnvalue_5 "QueryAndPhysics")
    (SplineMesh|SetStartandEnd _returnvalue_5 (Spline|GetLocationatDistanceAlongSpline _spline_2 (* _index (Variables|Default|GetMesh_length%20%28auto%20detect%29)) "Local") (Math|Vector|ClampVectorSize (Spline|GetTangentatDistanceAlongSpline _spline_2 (* _index (Variables|Default|GetMesh_length%20%28auto%20detect%29)) "Local") 0.0 (Variables|Default|GetMesh_length%20%28auto%20detect%29)) (Spline|GetLocationatDistanceAlongSpline _spline (* (+ _index 1) (Variables|Default|GetMesh_length%20%28auto%20detect%29)) "Local") (Math|Vector|ClampVectorSize (Spline|GetTangentatDistanceAlongSpline _spline (* (+ _index 1) (Variables|Default|GetMesh_length%20%28auto%20detect%29)) "Local") 0.0 (Variables|Default|GetMesh_length%20%28auto%20detect%29)) true :!class /Script/Engine.SplineMeshComponent)))