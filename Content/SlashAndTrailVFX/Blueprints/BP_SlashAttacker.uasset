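; BP_SlashAttacker is an attacker with a skeletal mesh that plays slash and dissolve visual effects.
; EnableSlash spawns a Niagara slash system at the hand_r socket, using its rotation with a roll offset.
; When the Disslove flag is set, DissolveStart and UndissolveStart each play a timeline that drives the DissolveAmount parameter on a dynamic instance of the mesh's first material.
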(event Custom|Dissolve%20Start
  (if (Variables|Default|GetDisslove)
    (bind _returnvalue (Rendering|Material|CreateDynamicMaterialInstance (Variables|Character|GetMesh) 0 0 "None" :!class /Script/Engine.PrimitiveComponent))
    (bind _value (Timeline|StartDissolve PlayFromStart)
      (:Update
        (Rendering|Material|SetScalarParameterValue _returnvalue "DissolveAmount" _value :!class /Script/Engine.MaterialInstanceDynamic)))))

(event Custom|Undissolve%20Start
  (if (Variables|Default|GetDisslove)
    (bind _returnvalue (Rendering|Material|CreateDynamicMaterialInstance (Variables|Character|GetMesh) 0 0 "None" :!class /Script/Engine.PrimitiveComponent))
    (bind _value (Timeline|StartUnDissolve PlayFromStart)
      (:Update
        (Rendering|Material|SetScalarParameterValue _returnvalue "DissolveAmount" _value :!class /Script/Engine.MaterialInstanceDynamic)))))

(event Custom|EnableSlash
  (bind _mesh (Variables|Character|GetMesh))
  (bind _returnvalue (Transformation|GetSocketTransform _mesh "hand_r" "RTS_World"))
  (Niagara|SpawnSystematLocation (Variables|Default|GetNiagaraSlash) (.location _returnvalue) (Math|Rotator|MakeRotator (+ (.roll (.rotation _returnvalue)) -9e+01) (.pitch (.rotation _returnvalue)) (.yaw (.rotation _returnvalue)))))

(fn ConstructionScript)