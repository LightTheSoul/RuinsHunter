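; BP_Angel_kneeing is an angel statue actor that shows an interaction prompt when the player is nearby.
; BeginPlay creates the UI_InterAction widget and hides the blue light particle system.
; InteractCollisionBox overlaps with the player pawn add or remove the widget and toggle the OverlappedWithStatue flag.
; The graph contains no interaction input and never turns the light back on.
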(event OnComponentBeginOverlap(Interactcollisionbox)
  (params (OverlappedComponent :type Primitive%20Component%20Object%20Reference) (OtherActor :type Actor%20Object%20Reference) (OtherComp :type Primitive%20Component%20Object%20Reference) (OtherBodyIndex :type Integer) (bFromSweep :type Boolean) (SweepResult :type Hit%20Result%20Structure%20%28by%20ref%29))
  (if (== OtherActor (Game|Player|GetPlayerPawn 0))
    (UserInterface|Viewport|AddtoViewport (Variables|Default|GetInteractWidget) 0)
    (Variables|Default|SetOverlappedWithStatue true)))

(event OnComponentEndOverlap(Interactcollisionbox)
  (params (OverlappedComponent :type Primitive%20Component%20Object%20Reference) (OtherActor :type Actor%20Object%20Reference) (OtherComp :type Primitive%20Component%20Object%20Reference) (OtherBodyIndex :type Integer))
  (bind _interactwidget (Variables|Default|GetInteractWidget))
  (if (== (Game|Player|GetPlayerPawn 0) OtherActor)
    (Utilities|IsValid _interactwidget
      (:Is%20Valid
        (Widget|RemovefromParent _interactwidget)
        (Variables|Default|SetOverlappedWithStatue false))
      (:Is%20Not%20Valid
        (Variables|Default|SetOverlappedWithStatue false)))))

(event EventBeginPlay
  (bind _returnvalue (UserInterface|CreateWidget "/Game/CustomContents/Widget/UI_InterAction.UI_InterAction_C"))
  (Variables|Default|SetInteractWidget _returnvalue)
  (bind _output_get (Variables|Default|SetBlueLight (Variables|Default|GetParticleSystem)))
  (Rendering|SetVisibility _output_get false false))

(fn ConstructionScript)